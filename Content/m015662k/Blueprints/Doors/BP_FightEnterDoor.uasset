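; BP_FightEnterDoor is a fight arena door that starts open, shuts when a fight begins and reopens when the fight volume is cleared.
; BindEvents hooks it to the supplied volume's fight-begin and cleared events, which drive the inherited door open, close and lock functions.
; A lock widget shows a text message during the fight.
; ResetDoor restores the unlocked, open state and hides that message.
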(event `self.ReceiveBeginPlay`
  (`parent.ReceiveBeginPlay`)
  (`self.OpenDoor`))

(event `Bind Events`
  (params (volume :type "/Game/m015662k/Blueprints/AI/Misc/BP_FightVolume Object Reference"))
  (add `/Game/m015662k/Blueprints/AI/Misc/BP_FightVolume.OnFightBegin` volume (delegate `Begin Fight`))
  (add `/Game/m015662k/Blueprints/AI/Misc/BP_FightVolume.OnVolumeCleared` volume (delegate `End Fight`)))

(event `Begin Fight`
  ;[1 1 1] Lock Doors
  (`self.CloseDoor` true)
  (message `/Game/m015662k/Assets/UI/Doors/BPI_DoorUI.ShowText` (`WidgetComponent.GetUserWidgetObject` (`self.Lock Widget`))))

(event `End Fight`
  ;[1 1 1] Unlock Doors
  (`self.SetLockState` false)
  (`self.OpenDoor`)
  (message `/Game/m015662k/Assets/UI/Doors/BPI_DoorUI.HideText` (`WidgetComponent.GetUserWidgetObject` (`self.Lock Widget`))))

(fn `ResetDoor`
  (`self.SetLockState` false)
  (`self.OpenDoor`)
  (message `/Game/m015662k/Assets/UI/Doors/BPI_DoorUI.HideText` (`WidgetComponent.GetUserWidgetObject` (`self.Lock Widget`))))

(fn `UserConstructionScript`
  (`parent.UserConstructionScript`))