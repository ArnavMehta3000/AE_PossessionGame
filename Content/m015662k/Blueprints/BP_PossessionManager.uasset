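; BP_PossessionManager is a player controller that switches possession between Viking, Cowboy and Soldier characters on three input actions and shows the mouse cursor.
; Its construction script caches the first actor found of each character class and of BP_CameraPawn.
; SetPossessCharacter unpossesses the current pawn, possesses the chosen one, then focuses and moves the shared camera pawn and sets it as the view target.
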(event `self.ReceiveBeginPlay`
  (set `self.bShowMouseCursor` true) ; Show mouse cursor
)

(event `InputAction|Character 1`
  (params (Key :type "Key Structure"))
  ;[1 1 1] Change possessed character
  (:`Pressed`
    (`self.SetPossessCharacter` (`self.vikingCharacter`))))

(event `InputAction|Character 2`
  (params (Key :type "Key Structure"))
  ;[1 1 1] Change possessed character
  (:`Pressed`
    (`self.SetPossessCharacter` (`self.cowboyCharacter`))))

(event `InputAction|Character 3`
  (params (Key :type "Key Structure"))
  ;[1 1 1] Change possessed character
  (:`Pressed`
    (`self.SetPossessCharacter` (`self.soldierCharacter`))))

(fn `SetPossessCharacter`
  (params (character :type "Pawn Object Reference"))
  (bind _camerapawn (`self.cameraPawn`))
  (`self.UnPossess`)
  (`/Engine/EditorBlueprintResources/StandardMacros.IsValid` character
    (:`Is Valid`
      (`self.Possess` character)
      (`/Game/m015662k/Blueprints/Camera/BP_CameraPawn.SetFocusedActor` _camerapawn character)
      (`/Game/m015662k/Blueprints/Camera/BP_CameraPawn.Move Camera` _camerapawn)
      (`self.SetViewTargetWithBlend` _camerapawn 0.0 "VTBlend_EaseInOut" 0.1))))

(fn `UserConstructionScript`
  (bind _outactors (`GameplayStatics.GetAllActorsOfClass` "/Game/m015662k/Characters/Blueprints/BP_Cowboy.BP_Cowboy_C"))
  (set `self.cowboyCharacter` (`|GetArrayItem` _outactors))
  (bind _outactors_2 (`GameplayStatics.GetAllActorsOfClass` "/Game/m015662k/Characters/Blueprints/BP_Viking.BP_Viking_C"))
  (set `self.vikingCharacter` (`|GetArrayItem` _outactors_2))
  (bind _outactors_3 (`GameplayStatics.GetAllActorsOfClass` "/Game/m015662k/Characters/Blueprints/BP_Soldier.BP_Soldier_C"))
  (set `self.soldierCharacter` (`|GetArrayItem` _outactors_3))
  (bind _outactors_4 (`GameplayStatics.GetAllActorsOfClass` "/Game/m015662k/Blueprints/Camera/BP_CameraPawn.BP_CameraPawn_C")) ; Get camera reference
  (set `self.cameraPawn` (`|GetArrayItem` _outactors_4)))