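; Gun component that fires hitscan shots from its owning actor using stored weapon data, apparently an unfinished prototype.
; SetWeaponData stores GunData, and FireWeapon runs one Visibility line trace per bullet, then sets CanFire.
; Each trace end combines owner rotation and axis vectors with random spread, used directly as a world position without adding the start location.
; Hits only print impact points with persistent debug lines, and Fire is an empty stub.
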(event `FireWeapon`
  (bind _returnvalue (`self.GetOwner`))
  (bind (_gundata_numofbullets _gundata_reloadtime _gundata_spread) (break `/Game/m015662k/Blueprints/Weapon/WeaponData` (`self.gunData`)))
  (bind _returnvalue_2 (`Actor.GetActorUpVector` _returnvalue))
  (bind (_returnvalue_roll _returnvalue_pitch _returnvalue_yaw) (`KismetMathLibrary.BreakRotator` (`Actor.K2_GetActorRotation` _returnvalue)))
  (for _ (range 1 (+ _gundata_numofbullets 1))
    (bind _output_get (set `self.direction` (* (`KismetMathLibrary.MakeVector` _returnvalue_roll _returnvalue_pitch _returnvalue_yaw) _returnvalue_2)))
    (bind _output_get_2 (set `self.perpDirection` (* (`KismetMathLibrary.Cross_VectorVector` (`Actor.GetActorRightVector` _returnvalue) _returnvalue_2) (`KismetMathLibrary.RandomFloatInRange` (* -1 _gundata_spread) _gundata_spread))))
    (bind _output_get_3 (set `self.finalDirection` (+ _output_get_2 _output_get)))
    (bind _outhit (`KismetSystemLibrary.LineTraceSingle` :`Start` (`Actor.K2_GetActorLocation` (`self.GetOwner`)) :`End` _output_get_3 :`TraceChannel` "TraceTypeQuery1" :`DrawDebugType` "Persistent"))
    (`KismetSystemLibrary.PrintString` (`KismetStringLibrary.Conv_VectorToString` (`.ImpactPoint` (`GameplayStatics.BreakHitResult` _outhit)))))
  (set `self.canFire` true))

(fn `Fire`
  (params (actor :type "Actor Object Reference")))

(fn `SetWeaponData`
  (params (weaponData :type "/Game/m015662k/Blueprints/Weapon/WeaponData Structure"))
  (set `self.gunData` weaponData))