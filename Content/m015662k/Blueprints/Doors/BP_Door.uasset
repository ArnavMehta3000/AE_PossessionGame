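; BP_Door is a two-panel sliding door that can be opened, closed and locked.
; The MoveDoor timeline lerps both panels' relative locations between the same StartPosition and EndPosition, playing from the start to open and reversing to close.
; OpenDoor runs only when unlocked, CloseDoor sets the lock state as it closes, and SetLockState changes the lock without moving the door.
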(event `Open`
  (bind (_direction _lerp_value) (`Timeline|MoveDoor` :!via `PlayFromStart` :!label _label) ; Timeline to open/close door
    (:`Update`
      (bind _returnvalue (`KismetMathLibrary.VLerp` (`self.startPosition`) (`self.endPosition`) _lerp_value))
      (`SceneComponent.K2_SetRelativeLocation` (`self.Door Left`) _returnvalue false false)
      (`SceneComponent.K2_SetRelativeLocation` (`self.Door Right`) _returnvalue false false))))

(event `Close`
  (goto _label :!via `Reverse`))

(fn `CloseDoor`
  (params (setLocked :type Boolean))
  (set `self.isLocked` setLocked)
  (`self.Close`))

(fn `OpenDoor`
  (if (not (`self.isLocked`))
    (`self.Open`)))

(fn `SetLockState`
  (params (lockState :type Boolean))
  (set `self.isLocked` lockState))

(fn `UserConstructionScript`)