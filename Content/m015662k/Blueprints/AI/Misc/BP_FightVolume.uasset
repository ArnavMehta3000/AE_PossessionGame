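; BP_FightVolume is a combat arena volume that signals its linked entry and exit doors when a fight begins and when the area is cleared.
; Both doors bind to the volume on BeginPlay, and a spawn trigger calls CloseLinkedDoors to broadcast the fight start.
; Bound enemies increment a counter and decrement it when killed.
; Clearing broadcasts only when the counter reaches zero and the box overlaps no enemies.
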(event `self.ReceiveBeginPlay`
  ;[1 1 1] Bind Events To Enter And Exit Doors
  (`/Game/m015662k/Blueprints/Doors/BP_FightEnterDoor.Bind Events` (`self.entryDoor`) self)
  (`/Game/m015662k/Blueprints/Doors/BP_FightExitDoor.Bind Events` (`self.exitDoor`) self))

(event `Close Linked Doors`
  ;[1 1 1] Called by spawn trigger
  (`self.OnFightBegin`))

(event `Bind Enemy To Volume`
  (params (actor :type "Actor Object Reference"))
  ;[1 1 1] Add Enemy To The Volume
  (bind _asenemy_base_bp (cast `/Game/m015662k/Characters/Blueprints/EnemyBase_BP` actor))
  (`self.AddEnemy`)
  (add `/Game/m015662k/Characters/Blueprints/EnemyBase_BP.OnKilled` _asenemy_base_bp (delegate `OnEnemyKilledInVolume`)))

(event `OnEnemyKilledInVolume`
  ;[1 1 1] Whenever Enemy is Killed
  (bind _currentenemycount (`self.RemoveEnemy`))
  (if (and (<= _currentenemycount 0) (<= (`KismetArrayLibrary.Array_Length` (`PrimitiveComponent.GetOverlappingActors` (`self.Box`) "/Game/m015662k/Characters/Blueprints/EnemyBase_BP.EnemyBase_BP_C")) 0))
    (`self.OnVolumeCleared`)))

(fn `AddEnemy`
  (returns (currentEnemyCount :type Integer))
  (bind _result (`/Engine/EditorBlueprintResources/StandardMacros.IncrementInt` (`self.enemiesInRoom`))
    (:`  `
      (return _result))))

(fn `RemoveEnemy`
  (returns (currentEnemyCount :type Integer))
  (bind _result (`/Engine/EditorBlueprintResources/StandardMacros.DecrementInt` (`self.enemiesInRoom`))
    (:`  `
      (return _result))))

(fn `UserConstructionScript`)