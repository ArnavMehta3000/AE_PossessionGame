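; BP_RoomSpawnTrigger is a box trigger that starts a delayed pass over a room's spawner list when a playable-looking character enters.
; Overlapping Soldier, Cowboy or Viking actors are added uniquely to PassedCharacters, whose count check passes from the first entry onward.
; After InitialDelay, a delayed loop steps through Spawners at DelayBetweenSpawn intervals, but its body has no actions.
; No once-only guard exists, so later overlaps can restart the sequence.
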(event `self.Box.OnComponentBeginOverlap`
  (params (OverlappedComponent :type "PrimitiveComponent Object Reference") (OtherActor :type "Actor Object Reference") (OtherComp :type "PrimitiveComponent Object Reference") (OtherBodyIndex :type Integer) (bFromSweep :type Boolean) (SweepResult :type "HitResult Structure (by ref)"))
  (bind _asbp_soldier (cast `/Game/m015662k/Characters/Blueprints/BP_Soldier` OtherActor)
    (:`then`
      (`KismetArrayLibrary.Array_AddUnique` (`self.passedCharacters`) _asbp_soldier))
    (:`CastFailed`
      (bind _asbp_cowboy (cast `/Game/m015662k/Characters/Blueprints/BP_Cowboy` OtherActor)
        (:`then`
          (`KismetArrayLibrary.Array_AddUnique` (`self.passedCharacters`) _asbp_cowboy))
        (:`CastFailed`
          (bind _asbp_viking (cast `/Game/m015662k/Characters/Blueprints/BP_Viking` OtherActor))
          (`KismetArrayLibrary.Array_AddUnique` (`self.passedCharacters`) _asbp_viking)))))
  (if (>= (`KismetArrayLibrary.Array_Length` (`self.passedCharacters`)) 1)
    (`KismetSystemLibrary.Delay` (`self.initialDelay`))
    (`/Game/m015662k/Blueprints/ActorMacros.For Each Loop With Delay` (`self.spawners`) (`self.delayBetweenSpawn`))))

(fn `UserConstructionScript`)