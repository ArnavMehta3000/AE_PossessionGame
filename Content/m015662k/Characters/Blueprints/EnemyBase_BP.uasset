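; Base enemy Blueprint that tracks health, fires a weapon and is destroyed on death.
; TakeDamage lowers health, updates the healthbar widget and calls the OnKilled dispatcher once at zero, which the enemy binds on BeginPlay to destroy itself.
; StartShooting and StopShooting events toggle fire on the character weapon component.
; A separate Kill function destroys the actor directly without calling OnKilled.
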(event `self.ReceiveBeginPlay`
  (set `self.currentHealth` (`self.maxHealth`))
  (add `self.OnKilled` (delegate `EnemyKilled`)))

(event `EnemyKilled`
  (`self.K2_DestroyActor`))

(event `StartShooting`
  (`/Game/m015662k/Blueprints/Weapon/CharacterWeaponComponent.Shoot` (`self.CharacterWeaponComponent`) true))

(event `StopShooting`
  (`/Game/m015662k/Blueprints/Weapon/CharacterWeaponComponent.Shoot` (`self.CharacterWeaponComponent`) false))

(fn `GetHealthPercent`
  (returns (percent :type "Float (double-precision)"))
  (return (/ (`self.currentHealth`) (`self.maxHealth`))))

(fn `Kill`
  (`self.K2_DestroyActor`))

(fn `TakeDamage`
  (params (damageAmount :type "Float (double-precision)"))
  (returns (currentHealth :type "Float (double-precision)"))
  (bind _output_get (set `self.currentHealth` (- (`self.currentHealth`) damageAmount)))
  (message `/Game/m015662k/Assets/UI/Misc/BPI_HealthBar.SetHealthPercent` (`WidgetComponent.GetUserWidgetObject` (`self.Healthbar Widget`)) (`self.GetHealthPercent`))
  (if (<= _output_get 0.0)
    (set `self.currentHealth` 0.0)
    (`/Engine/EditorBlueprintResources/StandardMacros.DoOnce` false
      (:`Completed`
        (`self.OnKilled`))))
  (return _output_get))

(fn `UserConstructionScript`)