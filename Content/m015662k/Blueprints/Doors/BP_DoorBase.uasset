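; Base Blueprint for a two-panel sliding door with a lock state.
; OpenDoor plays the MoveDoor timeline, lerping both panels between shared start and end relative positions, or shows the lock widget's text message if locked.
; CloseDoor sets the lock state and reverses the timeline, while SetLockState changes the lock alone.
; The lock message is hidden on BeginPlay, and ResetDoor is an empty stub.
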(event `self.ReceiveBeginPlay`
  (message `/Game/m015662k/Assets/UI/Doors/BPI_DoorUI.HideText` (`WidgetComponent.GetUserWidgetObject` (`self.Lock Widget`))))

(event `Open`
  (bind (_direction _lerp_value) (`Timeline|MoveDoor` :!via `PlayFromStart` :!label _label) ; Timeline to open/close door
    (:`Update`
      (bind _returnvalue (`KismetMathLibrary.VLerp` (`self.startPosition`) (`self.endPosition`) _lerp_value))
      (`SceneComponent.K2_SetRelativeLocation` (`self.Door Left`) _returnvalue false false)
      (`SceneComponent.K2_SetRelativeLocation` (`self.Door Right`) _returnvalue false false))))

(event `Close`
  (goto _label :!via `Reverse`))

(fn `CloseDoor`
  (params (setLocked :type Boolean))
  (set `self.isLocked` setLocked)
  (set `self.isOpen` false)
  (`self.Close`))

(fn `OpenDoor`
  (if (not (`self.isOpen`))
    (if (not (`self.isLocked`))
      (set `self.isOpen` true)
      (`self.Open`)
      (else
        (message `/Game/m015662k/Assets/UI/Doors/BPI_DoorUI.ShowText` (`WidgetComponent.GetUserWidgetObject` (`self.Lock Widget`))) ; Door locked, show text
      ))))

(fn `ResetDoor`)

(fn `SetLockState`
  (params (lockState :type Boolean))
  (set `self.isLocked` lockState))

(fn `UserConstructionScript`)