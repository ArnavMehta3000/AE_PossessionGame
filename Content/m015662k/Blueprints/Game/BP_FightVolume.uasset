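; Fight volume that runs an enemy encounter between an entry and exit door, broadcasting when the fight begins, clears or resets.
; Doors bind to the volume on BeginPlay, and a spawn trigger starts the fight.
; Registered enemies are counted down as they die until the volume clears.
; The construction script caches the Cowboy, Viking and Soldier; any one's death during a fight resets both doors and destroys remaining enemies.
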(event `self.ReceiveBeginPlay`
  ;[1 1 1] Bind Events To Enter And Exit Doors
  (`/Game/m015662k/Blueprints/Doors/BP_FightEnterDoor.Bind Events` (`self.entryDoor`) self)
  (`/Game/m015662k/Blueprints/Doors/BP_FightExitDoor.Bind Events` (`self.exitDoor`) self))

(event `Close Linked Doors`
  ;[1 1 1] Called by spawn trigger
  (`self.OnFightBegin`)
  (add `/Game/m015662k/Characters/Blueprints/PossessableCharacter_BP.OnPlayerKilled` (`self.cowboy`) (delegate `Cowboy Killed`))
  (add `/Game/m015662k/Characters/Blueprints/PossessableCharacter_BP.OnPlayerKilled` (`self.soldier`) (delegate `Viking Killed`))
  (add `/Game/m015662k/Characters/Blueprints/PossessableCharacter_BP.OnPlayerKilled` (`self.viking`) (delegate `Soldier Killed`)))

(event `Bind Enemy To Volume`
  (params (actor :type "Actor Object Reference"))
  ;[1 1 1] Add Enemy To The Volume
  (bind _asenemy_base_bp (cast `/Game/m015662k/Characters/Blueprints/EnemyBase_BP` actor))
  (`KismetArrayLibrary.Array_AddUnique` (`self.enemiesInRoom`) _asenemy_base_bp)
  (`self.AddEnemy`)
  (add `/Game/m015662k/Characters/Blueprints/EnemyBase_BP.OnKilled` _asenemy_base_bp (delegate `OnEnemyKilledInVolume`)))

(event `Cowboy Killed`
  (params (killedPlayer :type "/Game/m015662k/Characters/Blueprints/PossessableCharacter_BP Object Reference"))
  (bind _entrydoor (`self.entryDoor`))
  ;[1 1 1] Reset Fight Volume and Enemies
  (message `/Game/m015662k/Assets/UI/Doors/BPI_DoorUI.HideText` _entrydoor :!label _label)
  (`/Game/m015662k/Blueprints/Doors/BP_DoorBase.ResetDoor` _entrydoor)
  (`/Game/m015662k/Blueprints/Doors/BP_DoorBase.ResetDoor` (`self.exitDoor`))
  (for _array_element (`self.enemiesInRoom`)
    (`/Engine/EditorBlueprintResources/StandardMacros.IsValid` _array_element
      (:`Is Valid`
        (`self.K2_DestroyActor` _array_element))))
  (set `self.enemiesInRoomCount` 0)
  (`self.FightVolumeReset`))

(event `OnEnemyKilledInVolume`
  ;[1 1 1] Remove Enemy From Volume
  (bind _currentenemycount (`self.RemoveEnemy`))
  (if (<= _currentenemycount 0)
    (`self.OnVolumeCleared`)))

(event `Viking Killed`
  (params (killedPlayer :type "/Game/m015662k/Characters/Blueprints/PossessableCharacter_BP Object Reference"))
  ;[1 1 1] Reset Fight Volume and Enemies
  (goto _label))

(event `Soldier Killed`
  (params (killedPlayer :type "/Game/m015662k/Characters/Blueprints/PossessableCharacter_BP Object Reference"))
  ;[1 1 1] Reset Fight Volume and Enemies
  (goto _label))

(fn `AddEnemy`
  (returns (currentEnemyCount :type Integer))
  (bind _result (`/Engine/EditorBlueprintResources/StandardMacros.IncrementInt` (`self.enemiesInRoomCount`))
    (:`  `
      (return _result))))

(fn `RemoveEnemy`
  (returns (currentEnemyCount :type Integer))
  (bind _result (`/Engine/EditorBlueprintResources/StandardMacros.DecrementInt` (`self.enemiesInRoomCount`))
    (:`  `
      (return _result))))

(fn `UserConstructionScript`
  (bind _outactors (`GameplayStatics.GetAllActorsOfClass` "/Game/m015662k/Characters/Blueprints/BP_Cowboy.BP_Cowboy_C"))
  (set `self.cowboy` (`|GetArrayItem` _outactors))
  (bind _outactors_2 (`GameplayStatics.GetAllActorsOfClass` "/Game/m015662k/Characters/Blueprints/BP_Viking.BP_Viking_C"))
  (set `self.viking` (`|GetArrayItem` _outactors_2))
  (bind _outactors_3 (`GameplayStatics.GetAllActorsOfClass` "/Game/m015662k/Characters/Blueprints/BP_Soldier.BP_Soldier_C"))
  (set `self.soldier` (`|GetArrayItem` _outactors_3)))