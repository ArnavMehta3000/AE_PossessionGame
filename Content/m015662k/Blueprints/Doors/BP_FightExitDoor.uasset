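; Exit door for combat rooms that stays closed until the fight is cleared.
; On BeginPlay and on reset it closes and shows a "Clear Room To Unlock" message on its lock widget.
; BindEvents hooks a volume's OnVolumeCleared event to EndFight, which unlocks and opens the door and hides the message.
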(event `self.ReceiveBeginPlay`
  (bind _returnvalue (`WidgetComponent.GetUserWidgetObject` (`self.Lock Widget`)))
  (`parent.ReceiveBeginPlay`)
  (`self.CloseDoor` true)
  (message `/Game/m015662k/Assets/UI/Doors/BPI_DoorUI.UpdateText` _returnvalue "Clear Room To Unlock")
  (message `/Game/m015662k/Assets/UI/Doors/BPI_DoorUI.ShowText` _returnvalue))

(event `Bind Events`
  (params (volume :type "/Game/m015662k/Blueprints/Game/BP_FightVolume Object Reference"))
  (add `/Game/m015662k/Blueprints/Game/BP_FightVolume.OnVolumeCleared` volume (delegate `End Fight`)))

(event `End Fight`
  ;[1 1 1] Unlock Doors
  (`self.SetLockState` false)
  (`self.OpenDoor`)
  (message `/Game/m015662k/Assets/UI/Doors/BPI_DoorUI.HideText` (`WidgetComponent.GetUserWidgetObject` (`self.Lock Widget`))))

(fn `ResetDoor`
  (bind _returnvalue (`WidgetComponent.GetUserWidgetObject` (`self.Lock Widget`)))
  (`self.CloseDoor` true)
  (message `/Game/m015662k/Assets/UI/Doors/BPI_DoorUI.UpdateText` _returnvalue "Clear Room To Unlock")
  (message `/Game/m015662k/Assets/UI/Doors/BPI_DoorUI.ShowText` _returnvalue))

(fn `UserConstructionScript`
  (`parent.UserConstructionScript`))