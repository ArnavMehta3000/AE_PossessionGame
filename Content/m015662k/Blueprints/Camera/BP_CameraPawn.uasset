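; BP_CameraPawn is a spring-arm camera pawn that glides to a focused actor's location.
; SetFocusedActor stores the target, and the MoveCamera event replays FocusTimeline, whose curve drives a location lerp toward it.
; Each update lerps from the pawn's current location rather than a cached start and prints the result.
; The construction script caches the spring arm's default length, which is not used elsewhere in this file.
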(event `Move Camera`
  (bind (_direction _anim_curve) (`Timeline|Focus Timeline` :!via `PlayFromStart`)
    (:`Update`
      (bind _returnvalue (`KismetMathLibrary.VLerp` (`self.K2_GetActorLocation`) (`self.K2_GetActorLocation` (`self.focusedActor`)) _anim_curve))
      (`KismetSystemLibrary.PrintString` (`KismetStringLibrary.Conv_VectorToString` _returnvalue))
      (`self.K2_SetActorLocation` _returnvalue))))

(fn `SetFocusedActor`
  (params (focusedActor :type "Actor Object Reference"))
  (set `self.focusedActor` focusedActor))

(fn `UserConstructionScript`
  (set `self.defaultArmLength` (`SpringArmComponent.TargetArmLength` (`self.SpringArm`))))