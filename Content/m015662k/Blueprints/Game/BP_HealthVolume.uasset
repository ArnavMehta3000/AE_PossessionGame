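; BP_HealthVolume is a trigger volume that restores health to a PossessableCharacter_BP while it overlaps the box.
; On begin overlap it stores the character and starts a looping timer, which is cleared on end overlap.
; Each tick of the timer calls the character's TakeDamage with a negated HealthAddAmount, so healing reuses the damage function.
; Only one character reference and one timer handle are stored.
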(event `self.Box.OnComponentBeginOverlap`
  (params (OverlappedComponent :type "PrimitiveComponent Object Reference") (OtherActor :type "Actor Object Reference") (OtherComp :type "PrimitiveComponent Object Reference") (OtherBodyIndex :type Integer) (bFromSweep :type Boolean) (SweepResult :type "HitResult Structure (by ref)"))
  (bind _aspossessable_character_bp (cast `/Game/m015662k/Characters/Blueprints/PossessableCharacter_BP` OtherActor))
  (set `self.playerRef` _aspossessable_character_bp)
  (bind _returnvalue (`KismetSystemLibrary.K2_SetTimerDelegate` (delegate `Add health`) (`self.loopTime`) true))
  (set `self.timer` _returnvalue))

(event `Add health`
  ;[1 1 1] Add Health To The Player
  (`/Game/m015662k/Characters/Blueprints/PossessableCharacter_BP.TakeDamage` (`self.playerRef`) (* -1 (`self.healthAddAmount`))))

(event `self.Box.OnComponentEndOverlap`
  (params (OverlappedComponent :type "PrimitiveComponent Object Reference") (OtherActor :type "Actor Object Reference") (OtherComp :type "PrimitiveComponent Object Reference") (OtherBodyIndex :type Integer))
  ;[1 1 1] Stop Timer
  (cast `/Game/m015662k/Characters/Blueprints/PossessableCharacter_BP` OtherActor)
  (`KismetSystemLibrary.K2_ClearAndInvalidateTimerHandle` (`self.timer`)))

(fn `UserConstructionScript`)