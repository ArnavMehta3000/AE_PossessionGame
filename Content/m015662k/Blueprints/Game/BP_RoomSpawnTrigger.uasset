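; BP_RoomSpawnTrigger is a box trigger that starts a fight room encounter once enough distinct Soldier, Cowboy or Viking characters have passed through it.
; On reaching PassCount, a DoOnce closes the FightRoomVolume's linked doors, waits, then fires shuffled spawners at staggered intervals, binding each spawn to the volume.
; A volume reset re-arms the DoOnce and zeroes PassCount, so any one character's next overlap retriggers it.
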(event `self.ReceiveBeginPlay`
  ;[1 1 1] Reset Door binding
  (add `/Game/m015662k/Blueprints/Game/BP_FightVolume.FightVolumeReset` (`self.fightRoomVolume`) (delegate `Reset DoOnce`)))

(event `self.Box.OnComponentBeginOverlap`
  (params (OverlappedComponent :type "PrimitiveComponent Object Reference") (OtherActor :type "Actor Object Reference") (OtherComp :type "PrimitiveComponent Object Reference") (OtherBodyIndex :type Integer) (bFromSweep :type Boolean) (SweepResult :type "HitResult Structure (by ref)"))
  (bind _spawners (`self.spawners`))
  (bind _asbp_soldier (cast `/Game/m015662k/Characters/Blueprints/BP_Soldier` OtherActor)
    (:`then`
      (`KismetArrayLibrary.Array_AddUnique` (`self.passedCharacters`) _asbp_soldier))
    (:`CastFailed`
      (bind _asbp_cowboy (cast `/Game/m015662k/Characters/Blueprints/BP_Cowboy` OtherActor)
        (:`then`
          (`KismetArrayLibrary.Array_AddUnique` (`self.passedCharacters`) _asbp_cowboy))
        (:`CastFailed`
          (bind _asbp_viking (cast `/Game/m015662k/Characters/Blueprints/BP_Viking` OtherActor))
          (`KismetArrayLibrary.Array_AddUnique` (`self.passedCharacters`) _asbp_viking)))))
  (if (>= (`KismetArrayLibrary.Array_Length` (`self.passedCharacters`)) (`self.passCount`))
    (`/Engine/EditorBlueprintResources/StandardMacros.DoOnce` false :!label _label
      (:`Completed`
        (`/Game/m015662k/Blueprints/Game/BP_FightVolume.Close Linked Doors` (`self.fightRoomVolume`))
        (`KismetSystemLibrary.Delay` (`self.initialDelay`))
        (`KismetArrayLibrary.Array_Shuffle` _spawners)
        (bind _array_element (`/Game/m015662k/Blueprints/ActorMacros.For Each Loop With Delay` _spawners (`self.delayBetweenSpawn`))
          (:`Loop Body`
            (bind _spawnedactor (`/Game/m015662k/Blueprints/Game/BP_SpawnPoint.Spawn` _array_element))
            (`/Game/m015662k/Blueprints/Game/BP_FightVolume.Bind Enemy To Volume` (`self.fightRoomVolume`) _spawnedactor)))))))

(event `Reset DoOnce`
  (set `self.passCount` 0)
  (goto _label :!via `Reset`))

(fn `UserConstructionScript`
  (bind _outactors (`GameplayStatics.GetAllActorsOfClass` "/Game/m015662k/Blueprints/Camera/BP_CameraPawn.BP_CameraPawn_C")) ; Get camera reference
  (set `self.camera` (`|GetArrayItem` _outactors)))