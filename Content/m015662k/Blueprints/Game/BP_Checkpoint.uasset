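; Checkpoint actor that records a checkpoint position on possessable characters.
; When a PossessableCharacter_BP begins overlapping its Box, it writes the result of GetPosition into that character's CheckpointPosition.
; GetPosition offsets the checkpoint's X and Y randomly within RandomRange and uses a fixed Z height rather than the actor's own.
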(event `self.Box.OnComponentBeginOverlap`
  (params (OverlappedComponent :type "PrimitiveComponent Object Reference") (OtherActor :type "Actor Object Reference") (OtherComp :type "PrimitiveComponent Object Reference") (OtherBodyIndex :type Integer) (bFromSweep :type Boolean) (SweepResult :type "HitResult Structure (by ref)"))
  (bind _aspossessable_character_bp (cast `/Game/m015662k/Characters/Blueprints/PossessableCharacter_BP` OtherActor))
  (set `/Game/m015662k/Characters/Blueprints/PossessableCharacter_BP.checkpointPosition` (`self.GetPosition`) _aspossessable_character_bp))

(fn `GetPosition`
  (returns (position :type "Vector Structure"))
  (bind (_returnvalue_x _returnvalue_y) (`KismetMathLibrary.BreakVector` (`self.K2_GetActorLocation`)))
  (bind _randomrange (`self.randomRange`))
  (bind _randomrange_2 (`self.randomRange`))
  (return (`KismetMathLibrary.MakeVector` (+ _returnvalue_x (`KismetMathLibrary.RandomFloatInRange` (* -1 _randomrange_2) _randomrange_2)) (+ _returnvalue_y (`KismetMathLibrary.RandomFloatInRange` (* -1 _randomrange) _randomrange)) 100.0)))

(fn `UserConstructionScript`)